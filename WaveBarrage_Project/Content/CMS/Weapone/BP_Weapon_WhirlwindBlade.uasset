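; Whirlwind Blade weapon that periodically spawns BP_ProWhirlwindBlade projectiles around its owning character.
; A looping timer started on BeginPlay calls Fire every few seconds, which switches on WeaponLevel.
; Higher levels spawn more blades, growing from two to four to six, each targeting the owner and evenly spaced by a starting angle.
; The angle parameter is named as radians but receives degree-style values.
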(event Collision|EventActorBeginOverlap
  (params (OtherActor :type Actor%20Object%20Reference)))

(event EventTick
  (params (DeltaSeconds :type Float%20%28single-precision%29)))

(event EventBeginPlay
  (Utilities|Time|SetTimerbyFunctionName 0 "Fire" 3.0 true))

(fn ConstructionScript
  (|CallParentFunction))

(fn Fire
  (bind _ownercharacter (Variables|Default|GetOwnerCharacter))
  (bind _ownercharacter_2 (Variables|Default|GetOwnerCharacter))
  (bind _ownercharacter_3 (Variables|Default|GetOwnerCharacter))
  (bind _ownercharacter_4 (Variables|Default|GetOwnerCharacter))
  (bind _ownercharacter_5 (Variables|Default|GetOwnerCharacter))
  (bind _ownercharacter_6 (Variables|Default|GetOwnerCharacter))
  (bind _ownercharacter_7 (Variables|Default|GetOwnerCharacter))
  (bind _ownercharacter_8 (Variables|Default|GetOwnerCharacter))
  (bind _ownercharacter_9 (Variables|Default|GetOwnerCharacter))
  (bind _ownercharacter_10 (Variables|Default|GetOwnerCharacter))
  (bind _ownercharacter_11 (Variables|Default|GetOwnerCharacter))
  (bind _ownercharacter_12 (Variables|Default|GetOwnerCharacter))
  (switch int (Variables|Default|GetWeaponLevel)
    (:0
      (Game|SpawnActorfromClass "/Game/CMS/Weapone/BP_ProWhirlwindBlade.BP_ProWhirlwindBlade_C" (Transformation|GetActorTransform _ownercharacter_12) "Undefined" "MultiplyWithRoot" 0 _ownercharacter_12 0.0 0 :!label _label)
      (Game|SpawnActorfromClass "/Game/CMS/Weapone/BP_ProWhirlwindBlade.BP_ProWhirlwindBlade_C" (Transformation|GetActorTransform _ownercharacter_3) "Undefined" "MultiplyWithRoot" 0 _ownercharacter_3 1.8e+02 0))
    (:1
      (goto _label))
    (:2
      (goto _label))
    (:3
      (Game|SpawnActorfromClass "/Game/CMS/Weapone/BP_ProWhirlwindBlade.BP_ProWhirlwindBlade_C" (Transformation|GetActorTransform _ownercharacter) "Undefined" "MultiplyWithRoot" 0 _ownercharacter 0.0 0 :!label _label_2)
      (Game|SpawnActorfromClass "/Game/CMS/Weapone/BP_ProWhirlwindBlade.BP_ProWhirlwindBlade_C" (Transformation|GetActorTransform _ownercharacter_2) "Undefined" "MultiplyWithRoot" 0 _ownercharacter_2 1.8e+02 0)
      (Game|SpawnActorfromClass "/Game/CMS/Weapone/BP_ProWhirlwindBlade.BP_ProWhirlwindBlade_C" (Transformation|GetActorTransform _ownercharacter_9) "Undefined" "MultiplyWithRoot" 0 _ownercharacter_9 9e+01 0)
      (Game|SpawnActorfromClass "/Game/CMS/Weapone/BP_ProWhirlwindBlade.BP_ProWhirlwindBlade_C" (Transformation|GetActorTransform _ownercharacter_8) "Undefined" "MultiplyWithRoot" 0 _ownercharacter_8 2.7e+02 0))
    (:4
      (goto _label_2))
    (:5
      (Game|SpawnActorfromClass "/Game/CMS/Weapone/BP_ProWhirlwindBlade.BP_ProWhirlwindBlade_C" (Transformation|GetActorTransform _ownercharacter_4) "Undefined" "MultiplyWithRoot" 0 _ownercharacter_4 0.0 0)
      (Game|SpawnActorfromClass "/Game/CMS/Weapone/BP_ProWhirlwindBlade.BP_ProWhirlwindBlade_C" (Transformation|GetActorTransform _ownercharacter_5) "Undefined" "MultiplyWithRoot" 0 _ownercharacter_5 6e+01 0)
      (Game|SpawnActorfromClass "/Game/CMS/Weapone/BP_ProWhirlwindBlade.BP_ProWhirlwindBlade_C" (Transformation|GetActorTransform _ownercharacter_10) "Undefined" "MultiplyWithRoot" 0 _ownercharacter_10 1.2e+02 0)
      (Game|SpawnActorfromClass "/Game/CMS/Weapone/BP_ProWhirlwindBlade.BP_ProWhirlwindBlade_C" (Transformation|GetActorTransform _ownercharacter_11) "Undefined" "MultiplyWithRoot" 0 _ownercharacter_11 1.8e+02 0)
      (Game|SpawnActorfromClass "/Game/CMS/Weapone/BP_ProWhirlwindBlade.BP_ProWhirlwindBlade_C" (Transformation|GetActorTransform _ownercharacter_6) "Undefined" "MultiplyWithRoot" 0 _ownercharacter_6 2.4e+02 0)
      (Game|SpawnActorfromClass "/Game/CMS/Weapone/BP_ProWhirlwindBlade.BP_ProWhirlwindBlade_C" (Transformation|GetActorTransform _ownercharacter_7) "Undefined" "MultiplyWithRoot" 0 _ownercharacter_7 3e+02 0))))