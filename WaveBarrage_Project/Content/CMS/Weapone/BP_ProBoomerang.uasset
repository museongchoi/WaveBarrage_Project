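; Boomerang projectile actor that flies out along its attack direction and then returns, living for three seconds.
; Tick accumulates elapsed time, moving the actor forward for the first second and backward afterward.
; Movement is a fixed per-frame world offset without sweep or delta-time scaling, so its speed depends on frame rate and it has no collision handling.
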(event EventBeginPlay
  (Actor|SetLifeSpan 3.0))

(event Collision|EventActorBeginOverlap
  (params (OtherActor :type Actor%20Object%20Reference)))

(event EventTick
  (params (DeltaSeconds :type Float%20%28single-precision%29))
  (bind _output_get (Variables|Default|SetTime (+ DeltaSeconds (Variables|Default|GetTime))))
  (if (<= _output_get 1.0)
    (CallFunction|MoveForwad)
    (else
      (CallFunction|MoveBack))))

(fn ConstructionScript)

(fn MoveForwad
  (Transformation|AddActorWorldOffset (* (Variables|Default|GetAttackDirection) 1e+01)))

(fn MoveBack
  (Transformation|AddActorWorldOffset (* (Variables|Default|GetAttackDirection) -1e+01)))