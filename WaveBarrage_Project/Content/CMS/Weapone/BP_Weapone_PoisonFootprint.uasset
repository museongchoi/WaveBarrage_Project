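; BP_Weapone_PoisonFootprint is a weapon that periodically leaves poison footprints beneath its owning character.
; On BeginPlay it starts a looping timer that calls Fire.
; Fire requires the owner's BP_TopDownPlayerState, then spawns a BP_TestProPoisonFootprint at the projectile spawn point, offset downward on Z.
; A sum of player and weapon damage is left unconnected, so it is not passed to the spawned footprint.
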(event EventBeginPlay
  (|CallParentFunction)
  (Utilities|Time|SetTimerbyFunctionName 0 "Fire" 1.0 true))

(event Collision|EventActorBeginOverlap
  (params (OtherActor :type Actor%20Object%20Reference)))

(event EventTick
  (params (DeltaSeconds :type Float%20%28single-precision%29)))

(fn ConstructionScript
  (|CallParentFunction))

(fn Fire
  (bind _projectilespawnpoint (Variables|Default|GetProjectileSpawnPoint))
  (bind _returnvalue (Transformation|GetWorldLocation _projectilespawnpoint))
  (bind _asbp_top_down_player_state (Utilities|Casting|CastToBP_TopDownPlayerState (Variables|/Script/Engine.Pawn|GetPlayerState (Variables|Default|GetOwnerCharacter))))
  (Utilities|IsValid _asbp_top_down_player_state
    (:Is%20Valid
      (Game|SpawnActorfromClass "/Game/CMS/Weapone/BP_TestProPoisonFootprint.BP_TestProPoisonFootprint_C" (Math|Transform|MakeTransform (Math|Vector|MakeVector (.x _returnvalue) (.y _returnvalue) (- (.z _returnvalue) 1.4e+02)) "0, 0, 0" "1.000000,1.000000,1.000000") "Undefined" "MultiplyWithRoot" 0 0))))