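; CuteLauncher weapon Blueprint that auto-aims at nearby targets and periodically fires bursts of BP_ProCuteLauncher projectiles.
; A fast looping timer sphere-traces around the weapon, then turns it toward the closest actor of the hit actor's class, leaving pitch at zero.
; A slower timer starts Fire when idle, which uses another timer to spawn projectiles until reaching the weapon's count plus the owner PlayerState bonus.
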(event EventBeginPlay
  (Utilities|Time|SetTimerbyFunctionName 0 "CuteLauncherAutomaticAiming" 0.01 true)
  (Utilities|Time|SetTimerbyFunctionName 0 "CheckAttack" 2.0 true))

(fn ConstructionScript
  (|CallParentFunction))

(fn Fire
  (if (Variables|Auto|GetIsAttacking)
    (bind _ownercharacter (Variables|Default|GetOwnerCharacter)
      (:then
        (bind _asbp_top_down_player_state (Utilities|Casting|CastToBP_TopDownPlayerState (Variables|/Script/Engine.Pawn|GetPlayerState _ownercharacter)))
        (Variables|Default|SetMaxProjectileCnt (+ (Variables|Default|GetProjectileCount) (Variables|/Game/CMS/BP_TopDownPlayerState.BP_TopDownPlayerState_C|GetProjectileCounts _asbp_top_down_player_state)))
        (Utilities|Time|SetTimerbyFunctionName 0 "SpawnProjectile" 0.02 true))
      (:else))))

(fn SpawnProjectile
  (bind _projectilespawnpoint (Variables|Default|GetProjectileSpawnPoint))
  (Development|PrintString "CuteLauncher" true true "(R=1.000000,G=0.094240,B=0.000000,A=1.000000)" 6e+01)
  (Game|SpawnActorfromClass "/Game/CMS/Weapone/BP_ProCuteLauncher.BP_ProCuteLauncher_C" (Math|Transform|MakeTransform (Transformation|GetWorldLocation _projectilespawnpoint) (Transformation|GetWorldRotation _projectilespawnpoint) "1.000000,1.000000,1.000000") "Undefined" "MultiplyWithRoot" 0 0)
  (bind _output_get (Variables|Default|SetCurProjectileCnt (+ (Variables|Default|GetCurProjectileCnt) 1)))
  (if (>= _output_get (Variables|Default|GetMaxProjectileCnt))
    (Utilities|Time|ClearTimerbyFunctionName 0 "SpawnProjectile")
    (Variables|Default|SetCurProjectileCnt 0)
    (Variables|Auto|SetIsAttacking false)))

(fn CuteLauncherAutomaticAiming
  (bind _returnvalue (Transformation|GetActorLocation))
  (bind _outhit (Collision|SphereTraceByChannel _returnvalue _returnvalue 5e+02 "TraceTypeQuery3" false 0 "ForOneFrame"))
  (Utilities|IsValid (.HitActor (Collision|BreakHitResult _outhit))
    (:Is%20Valid
      (bind _outactors (Actor|GetAllActorsOfClass (Utilities|GetClass (.HitActor (Collision|BreakHitResult _outhit)))))
      (Variables|Auto|SetClosestDistance 99999.0)
      (Variables|Auto|SetSetClosestEnemy 0)
      (for _array_element _outactors
        (if (< (Transformation|GetDistanceTo _array_element self) (Variables|Auto|GetClosestDistance))
          (Variables|Auto|SetClosestDistance (Transformation|GetDistanceTo _array_element self))
          (Variables|Auto|SetSetClosestEnemy _array_element)
          (Transformation|SetActorRotation (Math|Rotator|MakeRotator (.roll (Math|Rotator|FindLookatRotation (Transformation|GetActorLocation) (Transformation|GetActorLocation (Variables|Auto|GetSetClosestEnemy)))) 0.0 (.yaw (Math|Rotator|FindLookatRotation (Transformation|GetActorLocation) (Transformation|GetActorLocation (Variables|Auto|GetSetClosestEnemy)))))))))))

(fn CheckAttack
  (if (not (Variables|Auto|GetIsAttacking))
    (Variables|Auto|SetIsAttacking true)
    (CallFunction|Fire)))