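; BP_OrbitWeapon is a weapon that periodically spawns BP_Orbit actors at the first player's pawn.
; A looping timer started on BeginPlay calls Fire, which spawns each orbit with the pawn's transform and passes it the pawn as TargetActor along with a Center position.
; Tick keeps Center updated to the pawn's current location.
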(event EventBeginPlay
  (Utilities|Time|SetTimerbyFunctionName 0 "Fire" 3.0 true))

(event Collision|EventActorBeginOverlap
  (params (OtherActor :type Actor%20Object%20Reference)))

(event EventTick
  (params (DeltaSeconds :type Float%20%28single-precision%29))
  (Variables|Default|SetCenter (Transformation|GetActorLocation (Game|Player|GetPlayerPawn 0))))

(fn ConstructionScript
  (|CallParentFunction))

(fn Fire
  (bind _returnvalue (Game|Player|GetPlayerPawn 0))
  (Game|SpawnActorfromClass "/Game/CMS/Weapone/BP_Orbit.BP_Orbit_C" (Transformation|GetActorTransform _returnvalue) "Undefined" "MultiplyWithRoot" 0 (Variables|Default|GetCenter) _returnvalue 0))