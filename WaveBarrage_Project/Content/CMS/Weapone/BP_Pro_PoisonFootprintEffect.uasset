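; Poison footprint effect actor that lasts five seconds and is set up as a damage-over-time hazard for monsters.
; When a BP_MonsterBase overlaps its Cylinder, it calls AddDamage at once, then after a delay starts a looping timer on that function.
; AddDamage passes TotalDamage to ApplyDamage but supplies no damaged actor.
; The timer is never explicitly cleared, and overlap end is not handled.
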(event OnComponentBeginOverlap(Cylinder)
  (params (OverlappedComponent :type Primitive%20Component%20Object%20Reference) (OtherActor :type Actor%20Object%20Reference) (OtherComp :type Primitive%20Component%20Object%20Reference) (OtherBodyIndex :type Integer) (bFromSweep :type Boolean) (SweepResult :type Hit%20Result%20Structure%20%28by%20ref%29))
  (bind _asbp_monster_base (Utilities|Casting|CastToBP_MonsterBase OtherActor))
  (Utilities|IsValid _asbp_monster_base
    (:Is%20Valid
      (CallFunction|AddDamage)
      (Utilities|FlowControl|Delay 1.5)
      (Utilities|Time|SetTimerbyFunctionName 0 "AddDamage" 1.5 true))))

(event EventBeginPlay
  (Actor|SetLifeSpan 5.0))

(fn ConstructionScript)

(fn AddDamage
  (bind _totaldamage (Variables|Default|GetTotalDamage))
  (Development|PrintString (Utilities|String|Append "dam" (Utilities|String|ToString(Float) _totaldamage)) false false "(R=0.000000,G=0.660000,B=1.000000,A=1.000000)" 6e+01)
  (Game|Damage|ApplyDamage 0 _totaldamage 0 0))