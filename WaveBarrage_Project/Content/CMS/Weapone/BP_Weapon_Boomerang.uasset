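; Boomerang weapon Blueprint that automatically fires bursts of BP_ProBoomerang projectiles.
; BeginPlay starts a looping timer on Fire, which launches a faster looping SpawnProjectile timer only when the projectile count is zero.
; SpawnProjectile spawns each boomerang at ProjectileSpawnPoint, passing its forward vector as AttackDirection.
; Once the count reaches MaxProjectileCnt, it clears its timer and resets the count for the next burst.
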(event EventBeginPlay
  (Utilities|Time|SetTimerbyFunctionName 0 "Fire" 1.0 true))

(event Collision|EventActorBeginOverlap
  (params (OtherActor :type Actor%20Object%20Reference)))

(event EventTick
  (params (DeltaSeconds :type Float%20%28single-precision%29)))

(fn ConstructionScript
  (|CallParentFunction))

(fn Fire
  (if (== (Variables|Default|GetCurProjectileCnt) 0)
    (Utilities|Time|SetTimerbyFunctionName 0 "SpawnProjectile" 0.1 true)))

(fn SpawnProjectile
  (bind _projectilespawnpoint (Variables|Default|GetProjectileSpawnPoint))
  (bind _returnvalue (Transformation|GetWorldTransform _projectilespawnpoint))
  (Game|SpawnActorfromClass "/Game/CMS/Weapone/BP_ProBoomerang.BP_ProBoomerang_C" (Math|Transform|MakeTransform (.location _returnvalue) (.rotation _returnvalue) "1.000000,1.000000,1.000000") "Undefined" "MultiplyWithRoot" 0 (Math|Vector|GetForwardVector _projectilespawnpoint) 0)
  (bind _result (Math|Integer|IncrementInt (Variables|Default|GetCurProjectileCnt))
    (:%20%20
      (if (>= _result (Variables|Default|GetMaxProjectileCnt))
        (Utilities|Time|ClearTimerbyFunctionName 0 "SpawnProjectile")
        (Variables|Default|SetCurProjectileCnt 0)))))