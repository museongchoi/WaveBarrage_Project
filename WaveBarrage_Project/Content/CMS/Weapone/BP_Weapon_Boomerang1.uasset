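; Boomerang weapon Blueprint that calls Fire on a looping timer from BeginPlay.
; When CurProjectileCnt is zero, Fire starts a faster looping timer on SpawnProjectile to launch a burst.
; SpawnProjectile is empty: its disconnected logic would spawn actors along ProjectileSpawnPoint's forward vector, then clear the timer and reset the count at MaxProjectileCnt.
; As wired, no projectiles spawn.
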(event EventBeginPlay
  (Utilities|Time|SetTimerbyFunctionName 0 "Fire" 1.0 true))

(event Collision|EventActorBeginOverlap
  (params (OtherActor :type Actor%20Object%20Reference)))

(event EventTick
  (params (DeltaSeconds :type Float%20%28single-precision%29)))

(fn ConstructionScript
  (|CallParentFunction))

(fn Fire
  (if (== (Variables|Default|GetCurProjectileCnt) 0)
    (Utilities|Time|SetTimerbyFunctionName 0 "SpawnProjectile" 0.1 true)))

(fn SpawnProjectile)