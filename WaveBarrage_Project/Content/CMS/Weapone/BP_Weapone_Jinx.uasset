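; BP_Weapone_Jinx is a weapon that fires a rapid burst of BP_Projectile actors from its projectile spawn point.
; Fire adds the owner's player-state ProjectileCounts to the weapon's base count, then starts a fast looping timer on SpawnProjectile.
; Each tick spawns one projectile; on reaching the total, it clears the timer, resets the counter, clears the owner's IsAttacking flag and calls its AttackFire.
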(event EventBeginPlay
  (|CallParentFunction))

(event Collision|EventActorBeginOverlap
  (params (OtherActor :type Actor%20Object%20Reference)))

(event EventTick
  (params (DeltaSeconds :type Float%20%28single-precision%29)))

(fn ConstructionScript
  (|CallParentFunction))

(fn Fire
  (bind _ownercharacter (Variables|Default|GetOwnerCharacter)
    (:then
      (bind _asbp_top_down_player_state (Utilities|Casting|CastToBP_TopDownPlayerState (Variables|/Script/Engine.Pawn|GetPlayerState _ownercharacter)))
      (Variables|Default|SetMaxProjectileCnt (+ (Variables|Default|GetProjectileCount) (Variables|/Game/CMS/BP_TopDownPlayerState.BP_TopDownPlayerState_C|GetProjectileCounts _asbp_top_down_player_state)))
      (Utilities|Time|SetTimerbyFunctionName 0 "SpawnProjectile" 0.02 true))
    (:else
      (Development|PrintString "Owner Character Not Valid"))))

(fn SpawnProjectile
  (bind _projectilespawnpoint (Variables|Default|GetProjectileSpawnPoint))
  (bind _ownercharacter (Variables|Default|GetOwnerCharacter))
  (Game|SpawnActorfromClass "/Game/CMS/BP_Projectile.BP_Projectile_C" (Math|Transform|MakeTransform (Transformation|GetWorldLocation _projectilespawnpoint) (Transformation|GetWorldRotation _projectilespawnpoint) "1.000000,1.000000,1.000000") "Undefined" "MultiplyWithRoot" 0 0)
  (bind _output_get (Variables|Default|SetCurProjectileCnt (+ (Variables|Default|GetCurProjectileCnt) 1)))
  (if (>= _output_get (Variables|Default|GetMaxProjectileCnt))
    (Utilities|Time|ClearTimerbyFunctionName 0 "SpawnProjectile")
    (Variables|Default|SetCurProjectileCnt 0)
    (Variables|/Game/CMS/BP_TopDownCharacter_CMS.BP_TopDownCharacter_CMS_C|SetIsAttacking _ownercharacter false)
    (Default|AttackFire _ownercharacter)))