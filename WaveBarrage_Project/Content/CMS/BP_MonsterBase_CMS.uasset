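; Base monster Blueprint that turns toward a target player and moves forward.
; Each tick it yaws its root at a set speed toward TargetPlayer's relative look-at angle, then offsets itself along its forward vector without sweep if CanMoveForward is true.
; CheckCanMoveForward sets that flag with a forward Visibility line trace.
; BeginPlay starts a timer by function name with no function specified, and TargetPlayer is not assigned here.
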(event EventBeginPlay
  (Utilities|Time|SetTimerbyFunctionName 0 "" 0.0))

(event Collision|EventActorBeginOverlap
  (params (OtherActor :type Actor%20Object%20Reference)))

(event EventTick
  (params (DeltaSeconds :type Float%20%28single-precision%29))
  (CallFunction|SpintoTargetPlayer)
  (CallFunction|MoveForward))

(fn ConstructionScript)

(fn MoveForward
  (if (Variables|Default|GetbCanMoveForward)
    (Transformation|AddActorWorldOffset (* (Transformation|GetActorForwardVector) (Variables|Default|GetSpeed)))))

(fn CheckCanMoveForward
  (bind _returnvalue (Transformation|GetActorLocation))
  (bind _returnvalue_2 (Collision|LineTraceByChannel _returnvalue (+ _returnvalue (* (Transformation|GetActorForwardVector) (Variables|Default|GetCheckDist))) "TraceTypeQuery1" false 0 "None"))
  (Variables|Default|SetbCanMoveForward (not _returnvalue_2)))

(fn SpintoTargetPlayer
  (bind _targetplayer (Variables|Default|GetTargetPlayer)
    (:then
      (if (not (Math|Float|NearlyEqual(Float) (.yaw (Math|Rotator|FindRelativeLookatRotation (Transformation|GetActorTransform) (Transformation|GetActorLocation _targetplayer))) 0.0 1e-06))
        (if (> (.yaw (Math|Rotator|FindRelativeLookatRotation (Transformation|GetActorTransform) (Transformation|GetActorLocation _targetplayer))) 0.0)
          (Transformation|AddRelativeRotation (Variables|Default|GetDefaultSceneRoot) (Math|Rotator|MakeRotator 0.0 0.0 (* (Utilities|Time|GetWorldDeltaSeconds) (Variables|Default|GetRotationSpeed))) false false)
          (else
            (Transformation|AddRelativeRotation (Variables|Default|GetDefaultSceneRoot) (Math|Rotator|MakeRotator 0.0 0.0 (* (Utilities|Time|GetWorldDeltaSeconds) (* (Variables|Default|GetRotationSpeed) -1.0))) false false)))))
    (:else)))