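; BP_Projectile is a projectile that expires after five seconds or is destroyed when its Sphere component hits something.
; On hit, it reads Damage from the first player's BP_TopDownPlayerState, truncates it and passes it to ApplyDamage, which has no damaged actor wired.
; If the player state cast fails, the projectile is not destroyed on hit.
; A random critical-hit chance check exists but is disconnected.
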(event OnComponentHit(Sphere)
  (params (HitComponent :type Primitive%20Component%20Object%20Reference) (OtherActor :type Actor%20Object%20Reference) (OtherComp :type Primitive%20Component%20Object%20Reference) (NormalImpulse :type Vector :default "0, 0, 0") (Hit :type Hit%20Result%20Structure%20%28by%20ref%29))
  (bind _asbp_top_down_player_state (Utilities|Casting|CastToBP_TopDownPlayerState (Variables|/Script/Engine.Controller|GetPlayerState (Game|GetPlayerController 0))))
  (Game|Damage|ApplyDamage 0 (Math|Conversions|ToFloat(Integer) (Math|Float|Truncate (Variables|/Game/CMS/BP_TopDownPlayerState.BP_TopDownPlayerState_C|GetDamage _asbp_top_down_player_state))) 0 0)
  (Actor|DestroyActor))

(event EventBeginPlay
  (Actor|SetLifeSpan 5.0))

(event Collision|EventActorBeginOverlap
  (params (OtherActor :type Actor%20Object%20Reference)))

(event EventTick
  (params (DeltaSeconds :type Float%20%28single-precision%29)))

(fn ConstructionScript)