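; BP_WeaponBasePGN is a weapon base for the top-down character that fires damage-carrying actors.
; SetPlayerReference casts the given character to cache its BP_TopDownPlayerState.
; Fire spawns a weapon-type actor at the supplied transform and passes it the computed damage.
; TotalDamage adds weapon damage divided by the product of player damage and level to the base, so that bonus shrinks as those stats grow.
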(event EventBeginPlay
  (Development|PrintString (Utilities|GetDisplayName (Variables|Default|GetPlayerState))))

(fn ConstructionScript)

(fn Fire
  (params (SpawnTranceForm :type Transform))
  (LocalVariables|SetSetSpawnTranceForm SpawnTranceForm)
  (bind _adddamage (CallFunction|TotalDamage))
  (Development|PrintString "Fire!!!!")
  (bind _returnvalue (Game|SpawnActorfromClass "/Game/CMS/Del_BP_WeapontypeBase.Del_BP_WeapontypeBase_C" SpawnTranceForm "Undefined" "MultiplyWithRoot" 0 0))
  (Default|AddDamage _returnvalue _adddamage))

(fn SetPlayerReference
  (params (Character :type Character%20Object%20Reference))
  (bind _output_get (Variables|Default|SetPlayerCharacter Character))
  (bind _asbp_top_down_character_cms_pgn (Utilities|Casting|CastToBP_TopDownCharacter_CMS_PGN _output_get))
  (bind _asbp_top_down_player_state (Utilities|Casting|CastToBP_TopDownPlayerState (Variables|/Script/Engine.Pawn|GetPlayerState _asbp_top_down_character_cms_pgn)))
  (Utilities|IsValid _asbp_top_down_player_state
    (:Is%20Valid
      (Variables|Default|SetPlayerState _asbp_top_down_player_state))))

(fn TotalDamage
  (bind _playerstate (Variables|Default|GetPlayerState))
  (return (+ (Variables|Default|GetWPDamage) (/ (Variables|Default|GetWPDamage) (* (Variables|/Game/CMS/BP_TopDownPlayerState.BP_TopDownPlayerState_C|GetDamage _playerstate) (Variables|/Game/CMS/BP_TopDownPlayerState.BP_TopDownPlayerState_C|GetPlayerLevel _playerstate))))))