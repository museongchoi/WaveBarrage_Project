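; Boomerang weapon that automatically throws volleys of BP_Boomerang projectiles from the player.
; A looping one-second timer calls Fire, which starts a faster SpawnProjectile timer when no volley count is in progress.
; Each spawn uses the player pawn's transform and forward vector as attack direction, incrementing a counter.
; At MaxProjectileCnt the spawn timer clears and the counter resets for the next volley.
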(event EventBeginPlay
  (|CallParentFunction)
  (Utilities|Time|SetTimerbyFunctionName 0 "Fire" 1.0 true))

(event Collision|EventActorBeginOverlap
  (params (OtherActor :type Actor%20Object%20Reference)))

(event EventTick
  (params (DeltaSeconds :type Float%20%28single-precision%29)))

(fn ConstructionScript
  (|CallParentFunction))

(fn Fire
  (if (== (Variables|Default|GetCurProjectileCnt) 0)
    (Utilities|Time|SetTimerbyFunctionName 0 "SpawnProjectile" 0.1 true)))

(fn SpawnProjectile
  (bind _returnvalue (Game|Player|GetPlayerPawn 0))
  (Game|SpawnActorfromClass "/Game/PGN/Blueprint/BP_Boomerang.BP_Boomerang_C" (Transformation|GetActorTransform _returnvalue) "Undefined" "MultiplyWithRoot" 0 (Transformation|GetActorForwardVector _returnvalue) 0)
  (bind _result (Math|Integer|IncrementInt (Variables|Default|GetCurProjectileCnt))
    (:%20%20
      (if (>= _result (Variables|Default|GetMaxProjectileCnt))
        (Utilities|Time|ClearTimerbyFunctionName 0 "SpawnProjectile")
        (Variables|Default|SetCurProjectileCnt 0)))))