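; BP_PGNHud manages the player's XP and level-up UI.
; On BeginPlay it adds a WBP_PGN_XP widget to the viewport and binds to the top-down character's LevelUpEvent.
; When that event signals a level-up, it reveals the XP widget's level-up border, adds a WBP_Boomerang widget, pauses the game and calls BindCard on the XP widget with a fixed index.
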(event EventBeginPlay
  (bind _returnvalue (UserInterface|CreateWidget "/Game/PGN/Blueprint/Widget/WBP_PGN_XP.WBP_PGN_XP_C"))
  (bind _output_get (Variables|Default|SetWidget _returnvalue))
  (UserInterface|Viewport|AddtoViewport _output_get 0)
  (CallFunction|LevelUpEvent))

(event Collision|EventActorBeginOverlap
  (params (OtherActor :type Actor%20Object%20Reference)))

(event EventTick
  (params (DeltaSeconds :type Float%20%28single-precision%29)))

(fn ConstructionScript)

(fn LevelUpEvent
  (bind _asbp_top_down_character_cms_pgn (Utilities|Casting|CastToBP_TopDownCharacter_CMS_PGN (Game|GetPlayerCharacter 0)))
  (EventDispatchers|BindEventtoLevelUpEvent _asbp_top_down_character_cms_pgn (EventDispatchers|CreateEvent :!event BPPGNHudAutoGenFunc)))

(fn BPPGNHudAutoGenFunc
  (params (LevelUp :type Boolean))
  (if LevelUp
    (Widget|SetVisibility (Variables|/Game/PGN/Blueprint/Widget/WBP_PGN_XP.WBP_PGN_XP_C|GetBorder_LevelUp (Variables|Default|GetWidget)) "Visible")
    (bind _returnvalue (UserInterface|CreateWidget "/Game/PGN/Blueprint/Widget/WBP_Boomerang.WBP_Boomerang_C" (Game|GetPlayerController 0)))
    (UserInterface|Viewport|AddtoViewport _returnvalue 0)
    (Game|SetGamePaused true)
    (Default|BindCard (Variables|Default|GetWidget))))