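; BP_Orbit is a short-lived actor that circles a target actor, removing itself two seconds after BeginPlay through its life span.
; Each Tick advances an angle by orbit speed and, while the target is valid, uses cosine and sine to place the actor at the orbit radius around the target's current XY position.
; The orbit stays at world Z zero regardless of the target's height, and moves without sweeping.
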(event EventBeginPlay
  (Actor|SetLifeSpan 2.0))

(event Collision|EventActorBeginOverlap
  (params (OtherActor :type Actor%20Object%20Reference)))

(event EventTick
  (params (DeltaSeconds :type Float%20%28single-precision%29))
  (bind _orbitradius (Variables|Default|GetOrbitRadius))
  (bind _output_get (Variables|Default|SetCurAngle (+ (Variables|Default|GetCurAngle) (* DeltaSeconds (Variables|Default|GetOrbitSpeed)))))
  (bind _targetactor (Variables|Default|GetTargetActor)
    (:then
      (Transformation|SetActorLocation (Math|Vector|MakeVector (+ (.x (Transformation|GetActorLocation _targetactor)) (* (Math|Trig|Cos(Radians) (Math|Trig|DegreesToRadians _output_get)) _orbitradius)) (+ (.y (Transformation|GetActorLocation _targetactor)) (* (Math|Trig|Sin(Radians) (Math|Trig|DegreesToRadians _output_get)) _orbitradius)) 0.0) false false))
    (:else)))

(fn ConstructionScript)