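; BP_PGNCharacter is a player character with Enhanced Input movement, look controls and a simple XP leveling system.
; BeginPlay adds the default mapping context, then move input follows control rotation and look input drives controller yaw and pitch.
; AddXp accumulates XP and, on reaching MaxXp, increments Level and resets XP to zero, discarding any overflow.
; The 3 key grants a fixed amount of XP through that event.
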(event Custom|AddXp
  (params (AddXp :type Float%20%28double-precision%29))
  (Variables|Default|SetXp (+ (Variables|Default|GetXp) AddXp))
  (if (>= (Variables|Default|GetXp) (Variables|Default|GetMaxXp))
    (Math|Integer|IncrementInt (Variables|Default|GetLevel)
      (:%20%20
        (Variables|Default|SetXp 0.0)))))

(event Input|EnhancedActionEvents|EnhancedInputActionIA_Move
  (params (ActionValue :type Vector%202D%20Structure) (ElapsedSeconds :type Float%20%28double-precision%29) (TriggeredSeconds :type Float%20%28double-precision%29) (InputAction :type Input%20Action%20Object%20Reference :default "/Game/PGN/Input/IA_Move.IA_Move"))
  (bind _returnvalue (Pawn|GetControlRotation :!class /Script/Engine.Pawn))
  (Pawn|Input|AddMovementInput (Math|Vector|GetRightVector (Math|Rotator|MakeRotator (.roll _returnvalue) 0.0 (.yaw _returnvalue))) (.x ActionValue) false)
  (Pawn|Input|AddMovementInput (Math|Vector|GetForwardVector (Math|Rotator|MakeRotator 0.0 0.0 (.yaw (Pawn|GetControlRotation :!class /Script/Engine.Pawn)))) (.y ActionValue) false))

(event Input|EnhancedActionEvents|EnhancedInputActionIA_Look
  (params (ActionValue :type Vector%202D%20Structure) (ElapsedSeconds :type Float%20%28double-precision%29) (TriggeredSeconds :type Float%20%28double-precision%29) (InputAction :type Input%20Action%20Object%20Reference :default "/Game/PGN/Input/IA_Look.IA_Look"))
  (Pawn|Input|AddControllerPitchInput (.y ActionValue))
  (Pawn|Input|AddControllerYawInput (.x ActionValue)))

(event EventBeginPlay
  (bind _returnvalue (Game|GetPlayerController 0))
  (bind _returnvalue_2 (PlayerController|LocalPlayerSubsystems|GetEnhancedInputLocalPlayerSubsystem _returnvalue))
  (Utilities|IsValid _returnvalue_2
    (:Is%20Valid
      (Input|AddMappingContext _returnvalue_2 "/Game/PGN/Input/IMC_PGNDefault.IMC_PGNDefault" 0 "(bIgnoreAllPressedKeysUntilRelease=True,bForceImmediately=False,bNotifyUserSettings=False)"))))

(event Input|KeyboardEvents|3
  (params (Key :type Key%20Structure :default "None"))
  (:Pressed
    (CallFunction|AddXp 1e+01)))

(fn ConstructionScript)