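; Game mode Blueprint that sets the weapon data table reference to DT_WeaponData on BeginPlay.
; It also holds a replicated Lev counter that appears to be test code: LevelTest increments and prints it.
; The Lev RepNotify reassigns the value to itself and prints it, while Tick and the construction script are empty.
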(event EventBeginPlay
  (Variables|Default|SetWeaponDataTable "/Game/DT_WeaponData.DT_WeaponData"))

(event EventTick
  (params (DeltaSeconds :type Float%20%28single-precision%29)))

(fn ConstructionScript)

(fn LevelTest
  (bind _result (Math|Integer|IncrementInt (Variables|Default|Getlev))
    (:%20%20
      (Development|PrintString (Utilities|String|ToString(Integer) _result)))))

(fn OnRepLev
  (bind _output_get (Variables|Default|Setlev (Variables|Default|Getlev)))
  (Development|PrintString (Utilities|String|ToString(Integer) _output_get)))