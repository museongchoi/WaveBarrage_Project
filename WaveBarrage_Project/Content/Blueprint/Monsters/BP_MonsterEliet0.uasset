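; BP_MonsterEliet0 is an elite monster Blueprint that shows its health on an on-screen widget.
; On BeginPlay it creates a WBP_ElietHp widget for the first player controller, passes itself as the monster, and adds it to the viewport.
; A looping timer then polls HP every tenth of a second and pushes it to the widget against a hard-coded maximum.
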(event EventBeginPlay
  (CallFunction|CreateHPWidget)
  (Utilities|Time|SetTimerbyFunctionName 0 "UpdateHp" 0.1 true))

(event Collision|EventActorBeginOverlap
  (params (OtherActor :type Actor%20Object%20Reference)))

(event EventTick
  (params (DeltaSeconds :type Float%20%28single-precision%29)))

(fn ConstructionScript)

(fn CreateHPWidget
  (bind _returnvalue (UserInterface|CreateWidget "/Game/PGN/Blueprint/Widget/MonsterWidget/WBP_ElietHp.WBP_ElietHp_C" (Game|GetPlayerController 0) self))
  (bind _output_get (Variables|Default|SetEliet0HpWidget _returnvalue))
  (UserInterface|Viewport|AddtoViewport _output_get 0))

(fn UpdateHp
  (Default|SetHp (Variables|Default|GetEliet0HpWidget) (Math|Conversions|ToFloat(Integer) (Variables|Default|GetHP)) 4e+03))