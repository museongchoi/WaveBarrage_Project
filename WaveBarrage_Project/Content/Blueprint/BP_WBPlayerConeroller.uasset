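; Player controller that sets up the XP HUD for the local player and relays a request to show card selection on level-up.
; On BeginPlay, the local controller creates and displays WBP_PGN_XP with its level-up border collapsed, then enables Game and UI input with a visible cursor.
; ShowCardSelectionWidget routes through the ResLevel client RPC, which calls CallLevleup on the owning client.
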(event Custom|ResLevel
  ;[1 1 1] client
  (Default|CallLevleup false))

(event EventBeginPlay
  (if (Pawn|IsLocalPlayerController)
    (bind _returnvalue (UserInterface|CreateWidget "/Game/PGN/Blueprint/Widget/WBP_PGN_XP.WBP_PGN_XP_C" (Game|GetPlayerController 0)))
    (bind _output_get (Variables|Default|SetWidget _returnvalue))
    (UserInterface|Viewport|AddtoViewport _output_get 0)
    (Variables|/Script/UMG.Widget|SetVisibility (Variables|/Game/PGN/Blueprint/Widget/WBP_PGN_XP.WBP_PGN_XP_C|GetBorder_LevelUp _output_get) "Collapsed")
    (Input|SetInputModeGameandUI self 0 "DoNotLock" true false)
    (Variables|Default|SetbShowMouseCursor true)))

(event EventTick
  (params (DeltaSeconds :type Float%20%28single-precision%29)))

(event EventShowCardSelectionWidget
  (CallFunction|ResLevel))

(fn ConstructionScript)